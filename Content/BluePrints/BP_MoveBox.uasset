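; BP_MoveBox is a moving obstacle that travels along a spline and launches the player character on overlap.
; On BeginPlay, the Animation timeline drives the Cube's position and rotation by distance along the spline, preserving its scale.
; A Box overlap with BP_Character launches it along the Arrow's forward vector, adding to its current velocity.
; The replay and reverse events are empty, and their calls never run.
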(event OnComponentBeginOverlap(Box)
  (params (OverlappedComponent :type Primitive%20Component%20Object%20Reference) (OtherActor :type Actor%20Object%20Reference) (OtherComp :type Primitive%20Component%20Object%20Reference) (OtherBodyIndex :type Integer) (bFromSweep :type Boolean) (SweepResult :type Hit%20Result%20Structure%20%28by%20ref%29))
  (bind _asbp_character (Utilities|Casting|CastToBP_Character OtherActor))
  (Character|LaunchCharacter _asbp_character (* 7e+02 (Math|Vector|GetForwardVector (Variables|Default|GetArrow))) false false))

(event Custom|Reverse%20Animation)

(event Custom|Play%20again)

(event EventBeginPlay
  (bind _spline (Variables|Default|GetSpline))
  (bind _animationalpha (Timeline|Animation PlayFromStart)
    (:Update
      (Transformation|SetWorldTransform (Variables|Default|GetCube) (Math|Transform|MakeTransform (Spline|GetLocationatDistanceAlongSpline _spline (* _animationalpha (Spline|GetSplineLength (Variables|Default|GetSpline))) "World") (Spline|GetRotationatDistanceAlongSpline _spline (* _animationalpha (Spline|GetSplineLength (Variables|Default|GetSpline))) "World") (Transformation|GetWorldScale (Variables|Default|GetCube))) false false))))

(fn ConstructionScript)