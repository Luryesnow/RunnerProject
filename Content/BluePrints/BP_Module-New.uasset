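; BP_Module-New is a spinning pickup module that advances the player's mechanic unlocks and opens a linked door.
; Tick rotates the Cube by a fixed yaw step each frame, without delta-time scaling.
; When BP_Character overlaps the Cube, it stores the capsule location as SaveLocationDoor and increments UnlockMechanics on the character.
; The module then destroys itself and calls StartOpenTheDoor on its referenced BP_Door.
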(event OnComponentBeginOverlap(Cube)
  (params (OverlappedComponent :type Primitive%20Component%20Object%20Reference) (OtherActor :type Actor%20Object%20Reference) (OtherComp :type Primitive%20Component%20Object%20Reference) (OtherBodyIndex :type Integer) (bFromSweep :type Boolean) (SweepResult :type Hit%20Result%20Structure%20%28by%20ref%29))
  (bind _asbp_character (Utilities|Casting|CastToBP_Character OtherActor))
  (Variables|/Game/BluePrints/BP_Character.BP_Character_C|SetSaveLocation_door _asbp_character (Transformation|GetWorldLocation (Variables|/Script/Engine.Character|GetCapsuleComponent _asbp_character)))
  (Math|Integer|IncrementInt (Variables|/Game/BluePrints/BP_Character.BP_Character_C|GetUnlock%20Mechanics _asbp_character)
    (:%20%20
      (Actor|DestroyActor)
      (bind _asbp_door (Utilities|Casting|CastToBP_Door (Variables|Default|GetDoor)))
      (Default|StartOpentheDoor _asbp_door))))

(event EventBeginPlay)

(event Collision|EventActorBeginOverlap
  (params (OtherActor :type Actor%20Object%20Reference)))

(event EventTick
  (params (DeltaSeconds :type Float%20%28single-precision%29))
  (Transformation|AddWorldRotation (Variables|Default|GetCube) "0,3.000000, 0" false false))

(fn ConstructionScript)