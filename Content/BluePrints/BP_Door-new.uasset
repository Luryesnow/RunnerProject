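; BP_Door-new is a sliding door Blueprint that opens and closes through two custom events.
; StartOpenthedoor plays the DoorMovement timeline, whose float track lerps the Door component's relative location along Y, and Closethedoor reverses it.
; Nothing in the file calls these events, as overlap and Tick are disabled.
; An unconnected leftover holds an alternate slide and a rotation lerp that never run.
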(event Custom|Start%20Open%20the%20door
  (bind _floatdoor (Timeline|DoorMovement Play)
    (:Update
      (Transformation|SetRelativeLocation (Variables|Default|GetDoor) (Math|Vector|Lerp(Vector) "0.000000,285.000000,0.000000" "0,100.000000, 0" _floatdoor) false false))))

(event Custom|Close%20the%20door
  (bind _floatdoor (Timeline|DoorMovement Reverse)
    (:Update
      (Transformation|SetRelativeLocation (Variables|Default|GetDoor) (Math|Vector|Lerp(Vector) "0.000000,285.000000,0.000000" "0,100.000000, 0" _floatdoor) false false))))

(event Collision|EventActorBeginOverlap
  (params (OtherActor :type Actor%20Object%20Reference)))

(event EventTick
  (params (DeltaSeconds :type Float%20%28single-precision%29)))

(fn ConstructionScript)