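; Cell receptacle that opens the elevator doors once the player has delivered all six cells.
; Cells start hidden with red lamps and lights.
; When BP_Character enters AreaOfAction, names in its CellsArray reveal matching cells once each, turn their indicators green, raise CountCells and decrement the character's collected count.
; Tick polls CountCells and, at six, calls OpenElevatorDoors on the first BP_Elevator_Doors after a short delay.
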(event OnComponentBeginOverlap(Areaofaction)
  (params (OverlappedComponent :type Primitive%20Component%20Object%20Reference) (OtherActor :type Actor%20Object%20Reference) (OtherComp :type Primitive%20Component%20Object%20Reference) (OtherBodyIndex :type Integer) (bFromSweep :type Boolean) (SweepResult :type Hit%20Result%20Structure%20%28by%20ref%29))
  (bind _asbp_character (Utilities|Casting|CastToBP_Character OtherActor))
  (Utilities|FlowControl|Delay 0.5)
  (for _array_element (Variables|/Game/BluePrints/BP_Character.BP_Character_C|GetCells%20Array _asbp_character)
    (Utilities|FlowControl|Sequence
      (:then_0
        (if (Utilities|Enum|Equal(Enum) _array_element "BP_Cell")
          (Utilities|FlowControl|DoOnce false
            (:Completed
              (Rendering|SetVisibility (Variables|Default|GetCell1) true false)
              (Rendering|Material|SetMaterial (Variables|Default|GetLamp%201) 0 "/Game/Materials_Project/M_Lamp_Green.M_Lamp_Green")
              (Rendering|Components|Light|SetLightColor (Variables|Default|GetPointLight1) "(R=0.000000,G=0.200000,B=0.000000,A=1.000000)" true)
              (Math|Integer|IncrementInt (Variables|Default|GetCountCells) :!label _label
                (:%20%20
                  (bind _outactors (Actor|GetAllActorsOfClass "/Game/BluePrints/BP_Character.BP_Character_C"))
                  (bind _asbp_character_2 (Utilities|Casting|CastToBP_Character (Utilities|Array|Get(acopy) _outactors)))
                  (Default|DecCellsCollected _asbp_character_2)))))))
      (:then_1
        (if (Utilities|Enum|Equal(Enum) _array_element "BP_Cell2")
          (Utilities|FlowControl|DoOnce false
            (:Completed
              (Rendering|SetVisibility (Variables|Default|GetCell2) true false)
              (Rendering|Material|SetMaterial (Variables|Default|GetLamp%202) 0 "/Game/Materials_Project/M_Lamp_Green.M_Lamp_Green")
              (Rendering|Components|Light|SetLightColor (Variables|Default|GetPointLight2) "(R=0.000000,G=0.200000,B=0.000000,A=1.000000)" true)
              (goto _label)))))
      (:then_2
        (if (Utilities|Enum|Equal(Enum) _array_element "BP_Cell3")
          (Utilities|FlowControl|DoOnce false
            (:Completed
              (Rendering|SetVisibility (Variables|Default|GetCell3) true false)
              (Rendering|Material|SetMaterial (Variables|Default|GetLamp%203) 0 "/Game/Materials_Project/M_Lamp_Green.M_Lamp_Green")
              (Rendering|Components|Light|SetLightColor (Variables|Default|GetPointLight3) "(R=0.000000,G=0.200000,B=0.000000,A=1.000000)" true)
              (goto _label)))))
      (:then_3
        (if (Utilities|Enum|Equal(Enum) _array_element "BP_Cell4")
          (Utilities|FlowControl|DoOnce false
            (:Completed
              (Rendering|SetVisibility (Variables|Default|GetCell4) true false)
              (Rendering|Material|SetMaterial (Variables|Default|GetLamp%204) 0 "/Game/Materials_Project/M_Lamp_Green.M_Lamp_Green")
              (Rendering|Components|Light|SetLightColor (Variables|Default|GetPointLight4) "(R=0.000000,G=0.200000,B=0.000000,A=1.000000)" true)
              (goto _label)))))
      (:then_4
        (if (Utilities|Enum|Equal(Enum) _array_element "BP_Cell5")
          (Utilities|FlowControl|DoOnce false
            (:Completed
              (Rendering|SetVisibility (Variables|Default|GetCell5) true false)
              (Rendering|Material|SetMaterial (Variables|Default|GetLamp%205) 0 "/Game/Materials_Project/M_Lamp_Green.M_Lamp_Green")
              (Rendering|Components|Light|SetLightColor (Variables|Default|GetPointLight5) "(R=0.000000,G=0.200000,B=0.000000,A=1.000000)" true)
              (goto _label)))))
      (:then_5
        (if (Utilities|Enum|Equal(Enum) _array_element "BP_Cell6")
          (Utilities|FlowControl|DoOnce false
            (:Completed
              (Rendering|SetVisibility (Variables|Default|GetCell6) true false)
              (Rendering|Material|SetMaterial (Variables|Default|GetLamp%206) 0 "/Game/Materials_Project/M_Lamp_Green.M_Lamp_Green")
              (Rendering|Components|Light|SetLightColor (Variables|Default|GetPointLight6) "(R=0.000000,G=0.200000,B=0.000000,A=1.000000)" true)
              (goto _label))))))))

(event EventBeginPlay
  (Rendering|Material|SetMaterial (Variables|Default|GetLamp%202) 0 "/Game/Materials_Project/M_Lamp_Red.M_Lamp_Red")
  (Rendering|SetVisibility (Variables|Default|GetCell1) false false)
  (Rendering|Components|Light|SetLightColor (Variables|Default|GetPointLight6) "(R=0.200000,G=0.000000,B=0.000000,A=1.000000)" true))

(event Collision|EventActorBeginOverlap
  (params (OtherActor :type Actor%20Object%20Reference)))

(event EventTick
  (params (DeltaSeconds :type Float%20%28single-precision%29))
  (if (== (Variables|Default|GetCountCells) 6)
    (Utilities|FlowControl|DoOnce false
      (:Completed
        (Utilities|FlowControl|Delay 0.5)
        (bind _outactors (Actor|GetAllActorsOfClass "/Game/BluePrints/BP_Elevator_Doors.BP_Elevator_Doors_C"))
        (bind _asbp_elevator_doors (Utilities|Casting|CastToBP_Elevator_Doors (Utilities|Array|Get(acopy) _outactors)))
        (Default|OpenElevatorDoors _asbp_elevator_doors)))))

(fn ConstructionScript)