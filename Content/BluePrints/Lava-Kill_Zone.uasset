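; Lava kill zone that teleports a BP_Character entering its box trigger back to a saved location.
; Characters moving faster than a speed threshold go to SaveLocationDoor, while slower ones alternate between SaveLocation and SaveLocation1 through a FlipFlop.
; The construction script positions and scales the box from Height and Size; matching logic for the Lava component is present but disconnected.
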(event OnComponentBeginOverlap(Box)
  (params (OverlappedComponent :type Primitive%20Component%20Object%20Reference) (OtherActor :type Actor%20Object%20Reference) (OtherComp :type Primitive%20Component%20Object%20Reference) (OtherBodyIndex :type Integer) (bFromSweep :type Boolean) (SweepResult :type Hit%20Result%20Structure%20%28by%20ref%29))
  (bind _asbp_character (Utilities|Casting|CastToBP_Character OtherActor))
  (Variables|Default|SetAs%20BP%20Character _asbp_character)
  (if (> (Math|Vector|VectorLength (Variables|/Script/Engine.MovementComponent|GetVelocity (Variables|/Script/Engine.Character|GetCharacterMovement (Variables|Default|GetAs%20BP%20Character)))) 3e+03)
    (Transformation|SetActorLocation (Variables|Default|GetAs%20BP%20Character) (Variables|/Game/BluePrints/BP_Character.BP_Character_C|GetSaveLocation_door (Variables|Default|GetAs%20BP%20Character)) false false)
    (else
      (Utilities|FlowControl|FlipFlop
        (:A
          (Transformation|SetActorLocation (Variables|Default|GetAs%20BP%20Character) (Variables|/Game/BluePrints/BP_Character.BP_Character_C|GetSaveLocation (Variables|Default|GetAs%20BP%20Character)) false false))
        (:B
          (Transformation|SetActorLocation (Variables|Default|GetAs%20BP%20Character) (Variables|/Game/BluePrints/BP_Character.BP_Character_C|GetSaveLocation_1 (Variables|Default|GetAs%20BP%20Character)) false false))))))

(event EventBeginPlay)

(event Collision|EventActorBeginOverlap
  (params (OtherActor :type Actor%20Object%20Reference)))

(event EventTick
  (params (DeltaSeconds :type Float%20%28single-precision%29)))

(fn ConstructionScript
  (bind _size (Variables|Default|GetSize))
  (Transformation|SetWorldTransform (Variables|Default|GetBox) (Math|Transform|MakeTransform (Math|Vector|MakeVector 0.0 0.0 (Variables|Default|GetHeight)) "0, 0, 0" (Math|Vector|MakeVector _size _size 1.0)) false false))