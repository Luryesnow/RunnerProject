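; BP_SplineBox is an actor that moves a cube along its spline, starting at BeginPlay.
; The AnimationAlpha timeline scales spline length to a distance, setting the cube's world location and rotation while keeping its scale.
; Timeline completion calls ReverseAnimation to play it backward.
; Each update also feeds a three-second Delay that calls PlayAgain, restarting the timeline from the start.
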(event Custom|Reverse%20Animation
  (bind _spline (Variables|Default|GetSpline))
  (bind _animationalpha (Timeline|AnimationAlpha Reverse)
    (:Update
      (Transformation|SetWorldTransform (Variables|Default|GetCube) (Math|Transform|MakeTransform (Spline|GetLocationatDistanceAlongSpline _spline (* _animationalpha (Spline|GetSplineLength (Variables|Default|GetSpline))) "World") (Spline|GetRotationatDistanceAlongSpline _spline (* _animationalpha (Spline|GetSplineLength (Variables|Default|GetSpline))) "World") (Transformation|GetWorldScale (Variables|Default|GetCube))) false false)
      (Utilities|FlowControl|Delay 3.0)
      (CallFunction|PlayAgain))
    (:Finished
      (CallFunction|ReverseAnimation))))

(event Custom|Play%20again
  (bind _spline (Variables|Default|GetSpline))
  (bind _animationalpha (Timeline|AnimationAlpha PlayFromStart)
    (:Update
      (Transformation|SetWorldTransform (Variables|Default|GetCube) (Math|Transform|MakeTransform (Spline|GetLocationatDistanceAlongSpline _spline (* _animationalpha (Spline|GetSplineLength (Variables|Default|GetSpline))) "World") (Spline|GetRotationatDistanceAlongSpline _spline (* _animationalpha (Spline|GetSplineLength (Variables|Default|GetSpline))) "World") (Transformation|GetWorldScale (Variables|Default|GetCube))) false false)
      (Utilities|FlowControl|Delay 3.0)
      (CallFunction|PlayAgain))
    (:Finished
      (CallFunction|ReverseAnimation))))

(event EventBeginPlay
  (bind _spline (Variables|Default|GetSpline))
  (bind _animationalpha (Timeline|AnimationAlpha PlayFromStart)
    (:Update
      (Transformation|SetWorldTransform (Variables|Default|GetCube) (Math|Transform|MakeTransform (Spline|GetLocationatDistanceAlongSpline _spline (* _animationalpha (Spline|GetSplineLength (Variables|Default|GetSpline))) "World") (Spline|GetRotationatDistanceAlongSpline _spline (* _animationalpha (Spline|GetSplineLength (Variables|Default|GetSpline))) "World") (Transformation|GetWorldScale (Variables|Default|GetCube))) false false)
      (Utilities|FlowControl|Delay 3.0)
      (CallFunction|PlayAgain))
    (:Finished
      (CallFunction|ReverseAnimation))))

(fn ConstructionScript)