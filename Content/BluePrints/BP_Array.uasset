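; BP_Array is an actor that appears to demonstrate array appending and iteration through a trigger box.
; Each overlap on the Box appends the current Number to Array, then loops over the whole array and prints every element on screen.
; It then increments Number and Index and prints an empty string as a separator; Index is not read elsewhere in the graph.
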(event OnComponentBeginOverlap(Box)
  (params (OverlappedComponent :type Primitive%20Component%20Object%20Reference) (OtherActor :type Actor%20Object%20Reference) (OtherComp :type Primitive%20Component%20Object%20Reference) (OtherBodyIndex :type Integer) (bFromSweep :type Boolean) (SweepResult :type Hit%20Result%20Structure%20%28by%20ref%29))
  (Utilities|Array|Add (Variables|Default|GetArray) (Variables|Default|GetNumber))
  (for _array_element (Variables|Default|GetArray)
    (Development|PrintString (Utilities|String|ToString(Integer) _array_element) true true "(R=0.000000,G=0.660000,B=1.000000,A=1.000000)" 5.0))
  (Math|Integer|IncrementInt (Variables|Default|GetNumber)
    (:%20%20
      (Math|Integer|IncrementInt (Variables|Default|GetIndex)
        (:%20%20
          (Development|PrintString " " true true "(R=0.000000,G=0.660000,B=1.000000,A=1.000000)" 5.0))))))

(event EventBeginPlay)

(event Collision|EventActorBeginOverlap
  (params (OtherActor :type Actor%20Object%20Reference)))

(event EventTick
  (params (DeltaSeconds :type Float%20%28single-precision%29)))

(fn ConstructionScript)