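; Swinging obstacle that knocks characters away when they overlap its side hit boxes.
; On BeginPlay, the Flow timeline swings the Cube through a yaw arc and rotates the left and right arrows alongside it.
; Both hit boxes launch characters along ArrowLeft's forward vector scaled by HitVelocity, leaving ArrowRight unused for launching.
; A separate DisableSaveBox sets SaveDisable on BP_Character while it overlaps that area.
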(event OnComponentBeginOverlap(BoxLeft)
  (params (OverlappedComponent :type Primitive%20Component%20Object%20Reference) (OtherActor :type Actor%20Object%20Reference) (OtherComp :type Primitive%20Component%20Object%20Reference) (OtherBodyIndex :type Integer) (bFromSweep :type Boolean) (SweepResult :type Hit%20Result%20Structure%20%28by%20ref%29))
  (bind _ascharacter (Utilities|Casting|CastToCharacter OtherActor))
  (Character|LaunchCharacter _ascharacter (* (Math|Vector|GetForwardVector (Variables|Default|GetArrowLeft)) (Variables|Default|GetHitVelocity)) false false))

(event OnComponentBeginOverlap(BoxRight)
  (params (OverlappedComponent :type Primitive%20Component%20Object%20Reference) (OtherActor :type Actor%20Object%20Reference) (OtherComp :type Primitive%20Component%20Object%20Reference) (OtherBodyIndex :type Integer) (bFromSweep :type Boolean) (SweepResult :type Hit%20Result%20Structure%20%28by%20ref%29))
  (bind _ascharacter (Utilities|Casting|CastToCharacter OtherActor))
  (Character|LaunchCharacter _ascharacter (* (Math|Vector|GetForwardVector (Variables|Default|GetArrowLeft)) (Variables|Default|GetHitVelocity)) false false))

(event OnComponentBeginOverlap(DisableSaveBox)
  (params (OverlappedComponent :type Primitive%20Component%20Object%20Reference) (OtherActor :type Actor%20Object%20Reference) (OtherComp :type Primitive%20Component%20Object%20Reference) (OtherBodyIndex :type Integer) (bFromSweep :type Boolean) (SweepResult :type Hit%20Result%20Structure%20%28by%20ref%29))
  (bind _asbp_character (Utilities|Casting|CastToBP_Character OtherActor))
  (Variables|/Game/BluePrints/BP_Character.BP_Character_C|SetSave%20Disable _asbp_character true))

(event OnComponentEndOverlap(DisableSaveBox)
  (params (OverlappedComponent :type Primitive%20Component%20Object%20Reference) (OtherActor :type Actor%20Object%20Reference) (OtherComp :type Primitive%20Component%20Object%20Reference) (OtherBodyIndex :type Integer))
  (bind _asbp_character (Utilities|Casting|CastToBP_Character OtherActor))
  (Variables|/Game/BluePrints/BP_Character.BP_Character_C|SetSave%20Disable _asbp_character false))

(event EventBeginPlay
  (bind _newtrack_0 (Timeline|Flow Play)
    (:Update
      (Transformation|SetRelativeRotation (Variables|Default|GetCube) (Math|Rotator|Lerp(Rotator) "-90.000000,0.000000, 0" "90.000000,0.000000,0.000000" _newtrack_0) false false)
      (Transformation|SetRelativeRotation (Variables|Default|GetArrowLeft) (Math|Rotator|Lerp(Rotator) "90.000000,0.000000,0.000000" "180.000000,0.000000,0.000000" _newtrack_0) false false)
      (Transformation|SetRelativeRotation (Variables|Default|GetArrowRight) (Math|Rotator|Lerp(Rotator) "0.000000,0.000000, 0" "90.000000,0.000000,0.000000" _newtrack_0) false false))))

(fn ConstructionScript)